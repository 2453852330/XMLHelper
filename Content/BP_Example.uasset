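; Example Blueprint that exercises an XMLHelper plugin's function library on BeginPlay by reading and writing XML files at hardcoded local paths.
; The read pass loads a sample document, walks child and sibling elements by key, and prints title, ID, person details and PosList element counts.
; The write pass builds a new document with top-level and nested text elements, then saves it to disk.
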(event EventBeginPlay
  (bind (_xmldocument _returnvalue) (Class|XMLBlueprintFunctionLibrary|BPLLoadXMLfromFile "D:\\\\Projects\\\\B1\\\\Plugins\\\\XMLHelper\\\\test_example\\\\example_01.xml"))
  (Utilities|FlowControl|Sequence
    (:then_0
      ;[1 1 1] read xml
      (if _returnvalue
        (Variables|Default|SetReadDoc _xmldocument)
        (Utilities|FlowControl|Sequence
          (:then_0
            (Development|PrintString (Utilities|String|Append "title : " (Class|XMLBlueprintFunctionLibrary|BPLGetElementText (Class|XMLBlueprintFunctionLibrary|BPLGetFirstChildElementfromElement (Class|XMLBlueprintFunctionLibrary|BPLGetRootElement (Variables|Default|GetReadDoc)))))))
          (:then_1
            (Development|PrintString (Utilities|String|Append "id : " (Class|XMLBlueprintFunctionLibrary|BPLGetElementText (Class|XMLBlueprintFunctionLibrary|BPLGetFirstChildElementfromElement (Class|XMLBlueprintFunctionLibrary|BPLGetRootElement (Variables|Default|GetReadDoc)) "ID")))))
          (:then_2
            (Development|PrintString (Utilities|String|Append "Name : " (Class|XMLBlueprintFunctionLibrary|BPLGetElementText (Class|XMLBlueprintFunctionLibrary|BPLGetFirstChildElementfromElement (Class|XMLBlueprintFunctionLibrary|BPLGetNextSiblingElement (Class|XMLBlueprintFunctionLibrary|BPLGetFirstChildElementfromElement (Class|XMLBlueprintFunctionLibrary|BPLGetRootElement (Variables|Default|GetReadDoc)) "ID")) "Name")) "     Age : " (Class|XMLBlueprintFunctionLibrary|BPLGetElementText (Class|XMLBlueprintFunctionLibrary|BPLGetFirstChildElementfromElement (Class|XMLBlueprintFunctionLibrary|BPLGetNextSiblingElement (Class|XMLBlueprintFunctionLibrary|BPLGetFirstChildElementfromElement (Class|XMLBlueprintFunctionLibrary|BPLGetRootElement (Variables|Default|GetReadDoc)) "ID")) "Age")))))
          (:then_3
            (Development|PrintString (Utilities|String|Append "null key : " (Utilities|String|ToString(Integer) (Class|XMLBlueprintFunctionLibrary|BPLGetCountfromElement (Class|XMLBlueprintFunctionLibrary|BPLGetFirstChildElementfromElement (Class|XMLBlueprintFunctionLibrary|BPLGetRootElement (Variables|Default|GetReadDoc)) "PosList"))) "     xpos key : " (Utilities|String|ToString(Integer) (Class|XMLBlueprintFunctionLibrary|BPLGetCountfromElement (Class|XMLBlueprintFunctionLibrary|BPLGetFirstChildElementfromElement (Class|XMLBlueprintFunctionLibrary|BPLGetRootElement (Variables|Default|GetReadDoc)) "PosList") "xpos"))))))))
    (:then_1
      ;[1 1 1] write xml
      (Variables|Default|SetWriteDoc (Class|XMLBlueprintFunctionLibrary|BPLCreateRootXML "HELLO"))
      (Utilities|FlowControl|Sequence
        (:then_0
          (Class|XMLBlueprintFunctionLibrary|BPLSetElementText (Class|XMLBlueprintFunctionLibrary|BPLInsertElementtoDocument (Variables|Default|GetWriteDoc) "World1") "this is world 1"))
        (:then_1
          (Class|XMLBlueprintFunctionLibrary|BPLSetElementText (Class|XMLBlueprintFunctionLibrary|BPLInsertElementtoDocument (Variables|Default|GetWriteDoc) "World2") "this is world 2"))
        (:then_2
          (bind _output_get (Variables|Default|SetmodelElement (Class|XMLBlueprintFunctionLibrary|BPLInsertElementtoDocument (Variables|Default|GetWriteDoc) "MODEL")))
          (Class|XMLBlueprintFunctionLibrary|BPLSetElementText (Class|XMLBlueprintFunctionLibrary|BPLInsertElementtoElement _output_get "mode1") "this is mode1"))
        (:then_3
          (Class|XMLBlueprintFunctionLibrary|BPLSetElementText (Class|XMLBlueprintFunctionLibrary|BPLInsertElementtoElement (Variables|Default|GetmodelElement) "mode2") "this is mode2"))
        (:then_4
          (Class|XMLBlueprintFunctionLibrary|BPLSaveXMLtoFile (Variables|Default|GetWriteDoc) "D:\\Projects\\B1\\Plugins\\XMLHelper\\test_example\\bp_write.xml"))))))

(fn ConstructionScript)